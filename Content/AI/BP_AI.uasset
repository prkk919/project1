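; Sword-wielding enemy AI character with a billboarded health bar that reacts to damage with hit montages, knockback, and ragdoll death before being destroyed.
; Its Attack function, returning a fixed duration, drives a three-montage combo advanced by AttackIndex and a saved-input flag.
; A looping-timer sphere trace along the blade damages "Damageable" actors with shake, sound and blood; a separate trace serves kicks.
; The stealth assassination function is unwired.
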(event `self.ReceiveBeginPlay`
  (bind _aswb_dummy_health (cast `/Game/Widget/WB_DummyHealth` (`WidgetComponent.GetWidget` (`self.Health Bar Widget`))))
  (set `self.HealthBar UI` _aswb_dummy_health))

(event `self.ReceiveTick`
  (params (DeltaSeconds :type "Float (single-precision)"))
  (bind _health_bar_widget (`self.Health Bar Widget`))
  (`SceneComponent.K2_SetWorldRotation` _health_bar_widget (`KismetMathLibrary.FindLookAtRotation` (`SceneComponent.K2_GetComponentLocation` _health_bar_widget) (`SceneComponent.K2_GetComponentLocation` (`PlayerCameraManager.TransformComponent` (`GameplayStatics.GetPlayerCameraManager` 0)))) false false))

(event `Ragdoll`
  ;[1 1 1] Ragdoll
  (`|ExecutionSequence`
    (:`then_0`
      (`KismetSystemLibrary.Delay` 2.5)
      (`PrimitiveComponent.SetSimulatePhysics` (`self.Mesh`) true))
    (:`then_1`
      (`KismetSystemLibrary.Delay` 1.7)
      (`GameplayStatics.PlaySoundAtLocation` "/Game/StarterContent/Audio/Fire01.Fire01" (`self.K2_GetActorLocation`) (struct) 1.0 1.0 0.0 null null null null))))

(event `self.ReceiveAnyDamage`
  (params (Damage :type "Float (single-precision)") (DamageType :type "DamageType Object Reference") (InstigatedBy :type "Controller Object Reference") (DamageCauser :type "Actor Object Reference"))
  (`self.PlayAnimMontage` (`|GetArrayItem` (`self.HitAnims`) (`KismetMathLibrary.RandomIntegerInRange` 0 (- (`KismetArrayLibrary.Array_Length` (`self.HitAnims`)) 1))))
  (bind _asbp_player (cast `/Game/Player/BP_Player` (`GameplayStatics.GetPlayerCharacter` 0)))
  (`self.LaunchCharacter` (* (`KismetMathLibrary.GetForwardVector` (`self.K2_GetActorRotation` _asbp_player)) 700.0))
  (`GameplayStatics.PlaySoundAtLocation` "/Game/Audio/MS_SwordHits.MS_SwordHits" (`self.K2_GetActorLocation`) (struct) 1.0 (`KismetMathLibrary.RandomFloatInRange` -1.0 2.0) 0.0 "/Game/Audio/SA_Character.SA_Character" null null null)
  (bind _isplayerdead_ (`/Game/Blueprints/BPC_PlayerState.Decrease Health` (`self.BPC_PlayerState`) Damage))
  (if _isplayerdead_
    (`PrimitiveComponent.SetCollisionObjectType` (`self.Mesh`) "ECC_PhysicsBody")
    (`PrimitiveComponent.SetSimulatePhysics` (`self.Mesh`) true)
    (`GameplayStatics.PlaySoundAtLocation` null (`self.K2_GetActorLocation`) (struct) 1.0 1.0 0.0 null null null null)
    (`SceneComponent.SetVisibility` (`self.Health Bar Widget`) false false)
    (`KismetSystemLibrary.Delay` 2.0)
    (`self.K2_DestroyActor`)))

(event `Attack1`
  ;[0.07819 0.07819 0.07819 0.3098] Combo Attack
  ;;[0.07819 0.07819 0.07819 0.3098] Attack1
  (`/Engine/EditorBlueprintResources/StandardMacros.DoOnce` false :!label _label
    (:`Completed`
      (`KismetSystemLibrary.Delay` 0.1)
      (`|PlayMontage` (`self.Mesh`) "/Game/Characters/Mannequins/Animations/SwordAttack/Attack1_Montage.Attack1_Montage"
        (:`then`
          (set `self.Attack Index` 1)
          (goto _label :!via `Reset`))))))

(event `Sword Attack Combo Call From BT`
  ;[0.07819 0.07819 0.07819 0.3098] Combo Attack
  ;;[0.07819 0.07819 0.07819 0.3098] Attack Input
  (if (`self.CanAttack?`)
    (`self.SwordAttack`)))

(event `Attack2`
  ;[0.07819 0.07819 0.07819 0.3098] Combo Attack
  ;;[0.07819 0.07819 0.07819 0.3098] Attack2
  (`/Engine/EditorBlueprintResources/StandardMacros.DoOnce` false :!label _label_2
    (:`Completed`
      (`KismetSystemLibrary.Delay` 0.1)
      (`|PlayMontage` (`self.Mesh`) "/Game/Characters/Mannequins/Animations/SwordAttack/Attack2_Montage.Attack2_Montage"
        (:`then`
          (set `self.Attack Index` 2)
          (goto _label_2 :!via `Reset`))))))

(event `SwordAttack`
  ;[0.07819 0.07819 0.07819 0.3098] Combo Attack
  ;;[0.07819 0.07819 0.07819 0.3098] Sword Attack
  (if (`self.IsAttacking?`)
    (set `self.SaveAttack?` true)
    (else
      (set `self.IsAttacking?` true)
      (switch `int` (`self.Attack Index`) :!label _label_3
        (:`0`
          (`self.Attack1`))
        (:`1`
          (`self.Attack2`))
        (:`2`
          (`self.Attack4`))))))

(event `Attack3`
  ;[0.07819 0.07819 0.07819 0.3098] Combo Attack
  ;;[0.07819 0.07819 0.07819 0.3098] Attack3 (Not Using At The Moment
  (`/Engine/EditorBlueprintResources/StandardMacros.DoOnce` false :!label _label_4
    (:`Completed`
      (`KismetSystemLibrary.Delay` 0.1)
      (`|PlayMontage` (`self.Mesh`) "/Game/Characters/Mannequins/Animations/SwordAttack/Kick_Montage.Kick_Montage"
        (:`then`
          (set `self.Attack Index` 3)
          (goto _label_4 :!via `Reset`))))))

(event `SwordAttackCombo`
  ;[0.07819 0.07819 0.07819 0.3098] Combo Attack
  ;;[0.07819 0.07819 0.07819 0.3098] Combo Continue
  (if (`self.SaveAttack?`)
    (set `self.SaveAttack?` false)
    (goto _label_3)
    (else
      (`self.StopCombo`))))

(event `Attack4`
  ;[0.07819 0.07819 0.07819 0.3098] Combo Attack
  ;;[0.07819 0.07819 0.07819 0.3098] Attack4
  (`/Engine/EditorBlueprintResources/StandardMacros.DoOnce` false :!label _label_5
    (:`Completed`
      (`KismetSystemLibrary.Delay` 0.1)
      (`|PlayMontage` (`self.Mesh`) "/Game/Characters/Mannequins/Animations/SwordAttack/Attack3_Montage.Attack3_Montage"
        (:`then`
          (set `self.Attack Index` 4)
          (goto _label_5 :!via `Reset`))))))

(event `StopCombo`
  ;[0.07819 0.07819 0.07819 0.3098] Combo Attack
  ;;[0.07819 0.07819 0.07819 0.3098] Stop Combo / Attack
  (set `self.IsAttacking?` false)
  (set `self.Attack Index` 0))

(event `StartSwordTrace`
  (bind _returnvalue (`KismetSystemLibrary.K2_SetTimerDelegate` (delegate `SwordTraceLoop`) 0.001 true))
  (set `self.SwordLoop` _returnvalue))

(event `SwordTraceLoop`
  (bind (_outhit _returnvalue) (`KismetSystemLibrary.SphereTraceSingle` :`Start` (`SceneComponent.K2_GetComponentLocation` (`self.SwordTopPoint`)) :`End` (`SceneComponent.K2_GetComponentLocation` (`self.SwordBottomPoint`)) :`Radius` 12.0 :`TraceChannel` "TraceTypeQuery1" :`DrawTime` 0.2))
  (if _returnvalue
    (bind (_bblockinghit _binitialoverlap _time _distance _location _impactpoint _normal _impactnormal _physmat _hitactor) (`GameplayStatics.BreakHitResult` _outhit))
    (if (`self.ActorHasTag` _hitactor "Damageable")
      (`/Engine/EditorBlueprintResources/StandardMacros.DoOnce` false :!label _label_6
        (:`Completed`
          (`GameplayStatics.ApplyDamage` _hitactor 3.0)
          (`GameplayStatics.PlayWorldCameraShake` "/Game/Blueprints/BP_SwordHitHandShake.BP_SwordHitHandShake_C" _location 0.0 2000.0)
          (`self.Play Sword Hit Sounds`)
          (`GameplayStatics.SpawnEmitterAtLocation` "/Game/FXs/Particles/Blood/P_Blood_Splat_Cone.P_Blood_Splat_Cone" _location (`KismetMathLibrary.MakeRotFromXY` _normal _normal) (1.6 1.6 1.6) true "AutoRelease")
          (`KismetSystemLibrary.Delay` 0.5)
          (goto _label_6 :!via `Reset`))))))

(event `SphereTrace`
  (bind _returnvalue (`SceneComponent.K2_GetComponentLocation` (`self.Sphere Trace`)))
  ;[0.07819 0.07819 0.07819 0.3098] Sphere Trace (For Step/Kick)
  (bind (_outhit _returnvalue_2) (`KismetSystemLibrary.SphereTraceSingle` :`Start` _returnvalue :`End` _returnvalue :`Radius` 25.0 :`TraceChannel` "TraceTypeQuery1" :`DrawTime` 0.2))
  (if _returnvalue_2
    (bind (_bblockinghit _binitialoverlap _time _distance _location _impactpoint _normal _impactnormal _physmat _hitactor) (`GameplayStatics.BreakHitResult` _outhit))
    (if (`self.ActorHasTag` _hitactor "Damageable")
      (`GameplayStatics.ApplyDamage` _hitactor 10.0)
      (`GameplayStatics.PlayWorldCameraShake` "/Game/Blueprints/BP_SwordHitHandShake.BP_SwordHitHandShake_C" _location 0.0 2000.0)
      (`self.Play Sword Hit Sounds`)
      (`GameplayStatics.SpawnEmitterAtLocation` "/Game/FXs/Particles/Blood/P_Blood_Splat_Cone.P_Blood_Splat_Cone" _location (`KismetMathLibrary.MakeRotFromXY` _normal _normal) (1.6 1.6 1.6) true "AutoRelease"))))

(event `StopSwordTrace`
  (`KismetSystemLibrary.K2_ClearAndInvalidateTimerHandle` (`self.SwordLoop`)))

(event `Play Sword Hit Sounds`
  ;[1 1 1] Play Sword Hit Sounds
  (`GameplayStatics.PlaySoundAtLocation` "/Game/Audio/MS_SwordHits.MS_SwordHits" (`self.K2_GetActorLocation` (`self.GetOwner`)) (struct) 1.0 1.0 0.0 null null null null))

(fn `Attack`
  (returns (`Animation Duration` :type "Float (double-precision)"))
  (`self.Sword Attack Combo Call From BT`)
  (return 0.4))

(fn `Stealth Back Assasin`
  (returns (`REF Location` :type "Vector Structure") (`Assasin Rotation` :type "Rotator Structure")))

(fn `UserConstructionScript`)