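; Actor component that tracks health and stamina for the player or an AI dummy and updates their UI bars.
; One tick after BeginPlay it casts the owner to BP_Player or BP_AI and picks the HUD or health bar widget.
; Decrease functions report depletion, while increase functions clamp or refill and write only to the player HUD.
; AddDamage separately lowers CurHP and fires a ChangeHp dispatcher with a fixed maximum.
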(event `self.ReceiveBeginPlay`
  (`KismetSystemLibrary.DelayUntilNextTick`)
  (bind _asbp_player (cast `/Game/Player/BP_Player` (`self.GetOwner`))
    (:`then`
      (set `self.Player Character BP` _asbp_player)
      (set `self.IsPlayer` true)
      (`ProgressBar.SetPercent` (`/Game/Widget/WB_HUD.StaminaBar` (`/Game/Player/BP_Player.WB HUD` (`self.Player Character BP`))) (/ (`self.Current Stamina`) (`self.Max Stamina`))))
    (:`CastFailed`
      (bind _asbp_ai (cast `/Game/AI/BP_AI` (`self.GetOwner`)))
      (set `self.Dummy BP` _asbp_ai)
      (set `self.IsPlayer` false)))
  (`ProgressBar.SetPercent` (select `bool` (`self.IsPlayer`) :`false` (`/Game/Widget/WB_DummyHealth.HealthBar` (`/Game/AI/BP_AI.HealthBar UI` (`self.Dummy BP`))) :`true` (`/Game/Widget/WB_HUD.HealthBar` (`/Game/Player/BP_Player.WB HUD` (`self.Player Character BP`)))) (/ (`self.Current Health`) (`self.Max Health`)))
  (`TextBlock.SetText` (select `bool` (`self.IsPlayer`) :`false` (`/Game/Widget/WB_DummyHealth.HealthText` (`/Game/AI/BP_AI.HealthBar UI` (`self.Dummy BP`))) :`true` (`/Game/Widget/WB_HUD.HealthText` (`/Game/Player/BP_Player.WB HUD` (`self.Player Character BP`)))) (`KismetTextLibrary.Conv_DoubleToText` (`self.Current Health`) "HalfToEven")))

(fn `AddDamage`
  (params (Damage :type "Float (double-precision)"))
  (bind _output_get (set `self.CurHP` (- (`self.CurHP`) Damage)))
  (`self.EventDispatcher_ChangeHp` _output_get 100.0))

(fn `Decrease Health`
  (params (Damage :type "Float (double-precision)"))
  (returns (`IsPlayerDead?` :type Boolean))
  (if (not (<= (`self.Current Health`) 0.0))
    (bind _output_get (set `self.Current Health` (- (`self.Current Health`) Damage)))
    (`ProgressBar.SetPercent` (select `bool` (`self.IsPlayer`) :`false` (`/Game/Widget/WB_DummyHealth.HealthBar` (`/Game/AI/BP_AI.HealthBar UI` (`self.Dummy BP`))) :`true` (`/Game/Widget/WB_HUD.HealthBar` (`/Game/Player/BP_Player.WB HUD` (`self.Player Character BP`)))) (/ _output_get (`self.Max Health`)))
    (`TextBlock.SetText` (select `bool` (`self.IsPlayer`) :`false` (`/Game/Widget/WB_DummyHealth.HealthText` (`/Game/AI/BP_AI.HealthBar UI` (`self.Dummy BP`))) :`true` (`/Game/Widget/WB_HUD.HealthText` (`/Game/Player/BP_Player.WB HUD` (`self.Player Character BP`)))) (`KismetTextLibrary.Conv_DoubleToText` (`self.Current Health`) "HalfToEven"))
    (if (<= (`self.Current Health`) 0.0)
      _
      (else
        (return false))))
  (return true))

(fn `Decrease Stamina`
  (params (`Stamina Deplete` :type "Float (double-precision)"))
  (returns (`Not Stamina Left` :type Boolean))
  (if (not (<= (`self.Current Stamina`) 0.0))
    (set `self.Current Stamina` (- (`self.Current Stamina`) `Stamina Deplete`))
    (`ProgressBar.SetPercent` (`/Game/Widget/WB_HUD.StaminaBar` (`/Game/Player/BP_Player.WB HUD` (`self.Player Character BP`))) (/ (`self.Current Stamina`) (`self.Max Stamina`)))
    (if (<= (`self.Current Stamina`) 0.0)
      _
      (else
        (return false))))
  (return true))

(fn `Increase Health`
  (params (`Added Health` :type "Float (double-precision)"))
  (bind _wb_hud (`/Game/Player/BP_Player.WB HUD` (`self.Player Character BP`)))
  (set `self.Current Health` (+ (`self.Current Health`) `Added Health`))
  (if (> (`self.Current Health`) (`self.Max Health`))
    (set `self.Current Health` (`self.Max Health`)))
  (`ProgressBar.SetPercent` (`/Game/Widget/WB_HUD.HealthBar` _wb_hud) (/ (`self.Current Health`) (`self.Max Health`)))
  (`TextBlock.SetText` (`/Game/Widget/WB_HUD.HealthText` _wb_hud) (`KismetTextLibrary.Conv_DoubleToText` (`self.Current Health`) "HalfToEven")))

(fn `Increase Max Health`
  (params (`Health Incrementation` :type "Float (double-precision)"))
  (bind _wb_hud (`/Game/Player/BP_Player.WB HUD` (`self.Player Character BP`)))
  (bind _output_get (set `self.Max Health` (+ (`self.Max Health`) `Health Incrementation`)))
  (set `self.Current Health` _output_get)
  (`ProgressBar.SetPercent` (`/Game/Widget/WB_HUD.HealthBar` _wb_hud) (/ (`self.Current Health`) (`self.Max Health`)))
  (`TextBlock.SetText` (`/Game/Widget/WB_HUD.HealthText` _wb_hud) (`KismetTextLibrary.Conv_DoubleToText` (`self.Current Health`) "HalfToEven")))

(fn `Increase Max Stamina`
  (params (`Added Stamina` :type "Float (double-precision)"))
  (bind _output_get (set `self.Current Stamina` (+ (`self.Max Stamina`) `Added Stamina`)))
  (set `self.Max Stamina` _output_get)
  (`ProgressBar.SetPercent` (`/Game/Widget/WB_HUD.StaminaBar` (`/Game/Player/BP_Player.WB HUD` (`self.Player Character BP`))) (/ (`self.Current Stamina`) (`self.Max Stamina`))))

(fn `Increase Stamina`
  (params (`Added Stamina` :type "Float (double-precision)"))
  (set `self.Current Stamina` (+ (`self.Current Stamina`) `Added Stamina`))
  (if (> (`self.Current Stamina`) (`self.Max Stamina`))
    (set `self.Current Stamina` (`self.Max Stamina`)))
  (`ProgressBar.SetPercent` (`/Game/Widget/WB_HUD.StaminaBar` (`/Game/Player/BP_Player.WB HUD` (`self.Player Character BP`))) (/ (`self.Current Stamina`) (`self.Max Stamina`))))